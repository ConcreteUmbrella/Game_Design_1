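; Button_BP is an interactable button that opens its paired door once the player character holds more than one key.
; On Interact, it checks the character's KeyCount, writes it back unchanged and prints an all-keys message.
; It then searches every BP_Door1 for a DoorValue matching its ButtonValue, opens the first match and switches the player's view target to that door.
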(event EventInteract
  (params (Player :type Character%20Object%20Reference))
  (bind _returnvalue (Actor|GetActorOfClass "/Game/Blueprints/BP_ThirdPersonCharacterCustom.BP_ThirdPersonCharacterCustom_C"))
  (bind _asbp_third_person_character_custom (Utilities|Casting|CastToBP_ThirdPersonCharacterCustom _returnvalue))
  (if (> (Variables|/Game/Blueprints/BP_ThirdPersonCharacterCustom.BP_ThirdPersonCharacterCustom_C|GetKey%20Count _asbp_third_person_character_custom) 1)
    (Variables|/Game/Blueprints/BP_ThirdPersonCharacterCustom.BP_ThirdPersonCharacterCustom_C|SetKey%20Count _asbp_third_person_character_custom (Variables|/Game/Blueprints/BP_ThirdPersonCharacterCustom.BP_ThirdPersonCharacterCustom_C|GetKey%20Count _asbp_third_person_character_custom))
    (Development|PrintString "You've got all of the keys, go push that button!")
    (bind _outactors (Actor|GetAllActorsOfClass "/Game/Blueprints/BP_Door1.BP_Door1_C"))
    (bind _array_element (Utilities|Array|ForEachLoopwithBreak _outactors :!label _label)
      (:LoopBody
        (if (== (Variables|/Game/Blueprints/BP_Door1.BP_Door1_C|GetDoor%20Value _array_element) (Variables|Default|GetButton%20Value))
          (Default|OpenDoor _array_element Player)
          (Game|Player|SetViewTargetwithBlend (Game|GetPlayerController 0) _array_element 0.0 "VTBlend_Linear" 0.0 false)
          (goto _label Break))))))

(fn ConstructionScript)