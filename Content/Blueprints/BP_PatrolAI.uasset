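; Patrol AI Blueprint that walks itself through actors tagged as patrol points for a test map.
; BeginPlay gathers the tagged actors, prints their count and starts GotoPatrolPoint, which uses AIMoveTo toward the current index.
; Success or failure prints a message, increments the index, waits briefly and calls GotoPatrolPoint again.
; The index never wraps, as the length check is unused and the shuffle never runs.
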(event Custom|Move%20to)

(event Custom|Go%20to%20Patrol%20Point
  (AI|AIMoveTo self (Transformation|GetActorLocation (Utilities|Array|Get(acopy) (stale EventBeginPlay _outactors) (Variables|Default|GetCurrentPatrolPoint))) 0 2e+02 false
    (:OnSuccess
      (Development|PrintString "Success"))
    (:OnFail
      (Development|PrintString "Failed to get to Destination")))
  (bind _result (Math|Integer|IncrementInt (Variables|Default|GetCurrentPatrolPoint))
    (:%20%20
      (Utilities|FlowControl|Delay 1.0)
      (CallFunction|GotoPatrolPoint))))

(event EventBeginPlay
  (bind _outactors (Actor|GetAllActorsOfClasswithTag "/Script/Engine.Actor" "PatrolPoint-TestMapNone"))
  (Development|PrintString (Utilities|String|Append "There are " (Utilities|String|ToString(Integer) (Utilities|Array|Length _outactors)) " patrol points"))
  (CallFunction|GotoPatrolPoint))

(fn ConstructionScript)